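; BP_Block_Destructible is a destructible block that can hide an exit or goodies.
; Destroy plays an explosion effect, spawns an exit block if flagged as the exit, otherwise a scaled-up goodies actor if flagged, then removes the block.
; HitAfterEnemyBombed recolors the mesh through a material parameter and sets the goodies flag, so the block yields goodies when later destroyed.
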(event `DestructInterface.Destroy`
  (`GameplayStatics.SpawnEmitterAtLocation` "/Game/StarterContent/Particles/P_Explosion.P_Explosion" (`self.K2_GetActorLocation`))
  (if (`self.bIsExitBlock`)
    (`|SpawnActorFromClass` "/Game/Game/Placables/Blocks/Block_ExitBlock.Block_ExitBlock_C" (`KismetMathLibrary.MakeTransform` (`self.K2_GetActorLocation`) (struct) (1.0 1.0 1.0)) "Undefined" "OverrideRootScale" null null)
    (elif (`self.bHasGoodies`)
      (`|SpawnActorFromClass` "/Game/Game/Placables/Goodies/BP_Goodines.BP_Goodines_C" (`KismetMathLibrary.MakeTransform` (`self.K2_GetActorLocation`) (struct) (1.8 1.8 1.8)) "Undefined" "OverrideRootScale" null null)))
  (`/Engine/EditorBlueprintResources/StandardMacros.IsValid` self
    (:`Is Valid`
      (`self.K2_DestroyActor`))))

(event `DestructInterface.HitAfterEnemyBombed`
  (`MeshComponent.SetVectorParameterValueOnMaterials` (`self.BlockMesh`) "Color" (`KismetMathLibrary.Conv_LinearColorToVector` (`self.Color`)))
  (set `self.bHasGoodies` true))

(fn `UserConstructionScript`)
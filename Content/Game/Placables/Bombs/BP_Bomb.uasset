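; Placeable bomb that, once Explode is called, waits on a short fuse, then checks for destructible blocks, spawns an explosion effect and destroys itself.
; Block detection runs in four perpendicular yaw directions out to TraceDistance, giving a cross-shaped blast.
; A sphere overlap toggles BombOverlapped on any BP_Enemy entering or leaving it.
; A ScaleBomb timeline for scaling the mesh exists but is never triggered.
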(event `BombInterface.Explode`
  (`KismetSystemLibrary.Delay` 3.0)
  (`self.DetectDestructibleBlocksInAllDirection` 0.0 (`self.TraceDistance`))
  (`self.DetectDestructibleBlocksInAllDirection` 90.0 (`self.TraceDistance`))
  (`self.DetectDestructibleBlocksInAllDirection` 180.0 (`self.TraceDistance`))
  (`self.DetectDestructibleBlocksInAllDirection` 270.0 (`self.TraceDistance`))
  (`GameplayStatics.SpawnEmitterAtLocation` "/Game/StarterContent/Particles/P_Explosion.P_Explosion" (`self.K2_GetActorLocation`))
  (`self.K2_DestroyActor`))

(event `self.Sphere.OnComponentBeginOverlap`
  (params (OverlappedComponent :type "PrimitiveComponent Object Reference") (OtherActor :type "Actor Object Reference") (OtherComp :type "PrimitiveComponent Object Reference") (OtherBodyIndex :type Integer) (bFromSweep :type Boolean) (SweepResult :type "HitResult Structure (by ref)"))
  (bind _asbp_enemy (cast `/Game/Game/EnemyAI/BP_Enemy` OtherActor))
  (set `Enemy.bBombOverlapped` true _asbp_enemy))

(event `self.Sphere.OnComponentEndOverlap`
  (params (OverlappedComponent :type "PrimitiveComponent Object Reference") (OtherActor :type "Actor Object Reference") (OtherComp :type "PrimitiveComponent Object Reference") (OtherBodyIndex :type Integer))
  (bind _asbp_enemy (cast `/Game/Game/EnemyAI/BP_Enemy` OtherActor))
  (set `Enemy.bBombOverlapped` false _asbp_enemy))

(fn `UserConstructionScript`)
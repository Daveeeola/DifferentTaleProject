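; Character Blueprint that sets up level width and grid size values from a referenced Blockout_Box when play begins.
; On BeginPlay it validates and casts that reference, takes the box's X and Y size as level widths and halves its blockout material grid size.
; It then calls InitializeVariables, which is defined outside this graph; the construction script is empty.
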(event `self.ReceiveBeginPlay`
  (bind _output (`|ConvertAsset` (`self.BlockoutBox`)))
  (`/Engine/EditorBlueprintResources/StandardMacros.IsValid` _output
    (:`Is Valid`
      (bind _asblockout_box (cast `/BlockoutToolsPlugin/Blueprints/Blockout_Box` _output))
      (bind (_boxsize_x _boxsize_y) (`KismetMathLibrary.BreakVector` (`/BlockoutToolsPlugin/Blueprints/Blockout_Box.BoxSize` _asblockout_box)))
      (set `self.LevelWidthX` _boxsize_x)
      (set `self.LevelWidthY` _boxsize_y)
      (set `self.GridSize` (/ (`BlockoutToolsParent.BlockoutMaterialGridSize` _asblockout_box) 2.0))
      (`self.InitializeVariables`))))

(fn `UserConstructionScript`)
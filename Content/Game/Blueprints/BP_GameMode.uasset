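; BP_GameMode is the game mode that tracks the high score and handles the end of a level, won or lost.
; On BeginPlay it caches the game instance and loads the stored high score from it.
; The game-over and game-won events save PlayerScore through the game instance if it beats that high score, then trigger the matching message on the first player's HUD.
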(event `self.ReceiveBeginPlay`
  (bind _output_get (set `self.BP Game Instance ` (`GameplayStatics.GetGameInstance`)))
  (bind _highscore (message `/Game/Game/SaveGame/BPI_GameInstance.Load High Score` _output_get))
  (set `self.HighScore` _highscore))

(event `self.GameOverEvent`
  (if (> (`self.PlayerScore`) (`self.HighScore`))
    (message `/Game/Game/SaveGame/BPI_GameInstance.SaveHighScore` (`self.BP Game Instance `) (`self.PlayerScore`)))
  (message `/Game/Game/UI/Interface/BPI_HUD.EventGameOver` (`PlayerController.GetHUD` (`GameplayStatics.GetPlayerController` 0))))

(event `Game Won Event`
  (if (> (`self.PlayerScore`) (`self.HighScore`))
    (message `/Game/Game/SaveGame/BPI_GameInstance.SaveHighScore` (`self.BP Game Instance `) (`self.PlayerScore`)))
  (message `/Game/Game/UI/Interface/BPI_HUD.EventPassedThisLevel` (`PlayerController.GetHUD` (`GameplayStatics.GetPlayerController` 0))))

(fn `UserConstructionScript`)
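; Grid-based enemy that picks open directions to move in and dies when hit by a bomb.
; On BeginPlay it takes level size and half the material grid size from a Blockout_Box, then uses them to find cell-centre locations.
; Four-way obstacle checks yield free directions for random selection, with long traces locating targets along them.
; A bomb hit runs four-way box checks, awards score, shows score text, hides the enemy and destroys it after a delay.
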(event `self.ReceiveBeginPlay`
  (bind _output (`|ConvertAsset` (`self.BlockoutBox`)))
  (`/Engine/EditorBlueprintResources/StandardMacros.IsValid` _output
    (:`Is Valid`
      (bind _asblockout_box (cast `/BlockoutToolsPlugin/Blueprints/Blockout_Box` _output))
      (bind (_boxsize_x _boxsize_y) (`KismetMathLibrary.BreakVector` (`/BlockoutToolsPlugin/Blueprints/Blockout_Box.BoxSize` _asblockout_box)))
      (set `self.LevelWidthX` _boxsize_x)
      (set `self.LevelWidthY` _boxsize_y)
      (set `self.GridSize` (/ (`BlockoutToolsParent.BlockoutMaterialGridSize` _asblockout_box) 2.0))
      (`self.InitializeVariables`))))

(event `self.CheckForBlockage`
  (`KismetArrayLibrary.Array_Clear` (`self.HitDirections`))
  (`KismetArrayLibrary.Array_Clear` (`self.NotHitDirections`))
  (`self.GetObstaclesInAllDirection` 0.0 "EET_Up")
  (`self.GetObstaclesInAllDirection` 90.0 "EET_Right")
  (`self.GetObstaclesInAllDirection` 180.0 "EET_Down")
  (`self.GetObstaclesInAllDirection` 270.0 "EET_Left")
  (for _array_element (`self.Directions`)
    (if (not (`KismetArrayLibrary.Array_Contains` (`self.HitDirections`) _array_element))
      (`KismetArrayLibrary.Array_AddUnique` (`self.NotHitDirections`) _array_element))))

(event `self.GetRandomSuitableDirection`
  (set `self.CurrentDirection` (`KismetArrayLibrary.Array_Random` (`self.NotHitDirections`))))

(event `CharInterface.OnBombHit`
  (`self.GetBoxesInAllFourDirections` 0.0)
  (`self.GetBoxesInAllFourDirections` 90.0)
  (`self.GetBoxesInAllFourDirections` 180.0)
  (`self.GetBoxesInAllFourDirections` 270.0)
  (message `GameModeInterface.AddScore` (`GameplayStatics.GetGameMode`) 100)
  (`SceneComponent.SetVisibility` (`self.ScoreText1`) true false)
  (`SceneComponent.SetVisibility` (`self.StaticMesh`) false false)
  (`PrimitiveComponent.SetCollisionEnabled` (`self.CapsuleComponent`) "NoCollision")
  (`KismetSystemLibrary.Delay` 2.0)
  (`self.K2_DestroyActor`))

(fn `GetAiMiddleLocation`
  (params (InDirection :type "EEDirectionToGo Enum" :default "EET_Up"))
  (returns (OutMiddleLocation :type "Vector Structure") (OutDirectionToGo :type "EEDirectionToGo Enum"))
  (bind (_location _direction) (`self.GetMiddleOfPlayerLocation`))
  (return _location _direction))

(fn `GetCurrentDirection`
  (returns (OutCurrentDirection :type "EEDirectionToGo Enum"))
  (`self.CheckForBlockage`)
  (`self.GetRandomSuitableDirection`)
  (return (`self.CurrentDirection`)))

(fn `GetLocationAtTraceAtFreeDirection`
  (params (Direction :type "EEDirectionToGo Enum" :default "EET_Up"))
  (returns (Location :type "Vector Structure") (bHit :type Boolean))
  (bind (_hitlocation _bhit) (`self.LocationAtTraceAlongDirection` Direction 15000.0))
  (return _hitlocation _bhit))

(fn `GetMiddleOfPlayerLocation`
  (returns (Location :type "Vector Structure") (Direction :type "EEDirectionToGo Enum"))
  (bind _gridsize (`self.GridSize`))
  (bind _output (`|ConvertAsset` (`self.BlockoutBox`)))
  (bind (_returnvalue_x _returnvalue_y) (`KismetMathLibrary.BreakVector` (`KismetMathLibrary.MakeVector` (.x (- (`self.K2_GetActorLocation`) (`self.K2_GetActorLocation` _output))) (.y (- (`self.K2_GetActorLocation`) (`self.K2_GetActorLocation` _output))))))
  (`/Engine/EditorBlueprintResources/StandardMacros.IsValid` _output
    (:`Is Valid`
      (return (+ (`self.K2_GetActorLocation` (`|ConvertAsset` (`self.BlockoutBox`))) (`KismetMathLibrary.MakeVector` (* (+ (`KismetMathLibrary.Conv_IntToDouble` (`KismetMathLibrary.FTrunc` (/ _returnvalue_x _gridsize))) 0.5) (`self.GridSize`)) (* (+ (`KismetMathLibrary.Conv_IntToDouble` (`KismetMathLibrary.FTrunc` (/ _returnvalue_y _gridsize))) 0.5) (`self.GridSize`)) (.z (`self.K2_GetActorLocation`)))) (`self.CurrentDirection`)))))

(fn `UserConstructionScript`
  (`SceneComponent.SetVisibility` (`self.ScoreText1`) false false))